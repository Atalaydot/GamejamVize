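; Teleport trigger actor with two overlap boxes that react only to the first-person character.
; While its flag is set, Box teleports the player to a fixed world position, then after a short delay plays a sound and calls the character's second text function.
; Box1 clears that flag, then once only calls the third text function and plays another sound after a delay before destroying the actor.
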(event `self.Box.OnComponentBeginOverlap`
  (params (OverlappedComponent :type "PrimitiveComponent Object Reference") (OtherActor :type "Actor Object Reference") (OtherComp :type "PrimitiveComponent Object Reference") (OtherBodyIndex :type Integer) (bFromSweep :type Boolean) (SweepResult :type "HitResult Structure (by ref)"))
  (if (stale `self.Box1.OnComponentBeginOverlap` _output_get)
    (bind _asbp_first_person_character (cast `/Game/FirstPerson/Blueprints/BP_FirstPersonCharacter` OtherActor))
    (`self.K2_SetActorLocation` _asbp_first_person_character (750.0 1450.0 200.0) false true)
    (`KismetSystemLibrary.Delay` 0.5)
    (`GameplayStatics.PlaySoundAtLocation` "/Game/speak/3.3" (`self.K2_GetActorLocation`) (struct) 1.0 1.0 0.0 null null null null)
    (`/Game/FirstPerson/Blueprints/BP_FirstPersonCharacter.secentmetin` _asbp_first_person_character)))

(event `self.Box1.OnComponentBeginOverlap`
  (params (OverlappedComponent :type "PrimitiveComponent Object Reference") (OtherActor :type "Actor Object Reference") (OtherComp :type "PrimitiveComponent Object Reference") (OtherBodyIndex :type Integer) (bFromSweep :type Boolean) (SweepResult :type "HitResult Structure (by ref)"))
  (bind _asbp_first_person_character (cast `/Game/FirstPerson/Blueprints/BP_FirstPersonCharacter` OtherActor))
  (bind _output_get (set `self.NewVar` false))
  (`/Engine/EditorBlueprintResources/StandardMacros.DoOnce` false
    (:`Completed`
      (`KismetSystemLibrary.Delay` 0.5)
      (`/Game/FirstPerson/Blueprints/BP_FirstPersonCharacter.thirdmetin` _asbp_first_person_character)
      (`GameplayStatics.PlaySoundAtLocation` "/Game/speak/4.4" (`self.K2_GetActorLocation`) (struct) 1.0 1.0 0.0 null null null null)
      (`KismetSystemLibrary.Delay` 3.0)
      (`self.K2_DestroyActor`))))

(fn `UserConstructionScript`)