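; Sliding door Blueprint that opens when the first-person character is inside its trigger box moving faster than a speed threshold.
; An overlap flag makes Tick repeat the speed check, and a Timeline lowers the Cube along Z, reversing when the character leaves.
; Door sounds play at the world origin, while the first overlap also triggers a delayed sound at the actor and calls the character's 7metin.
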(event `self.ReceiveBeginPlay`)

(event `self.ReceiveTick`
  (params (DeltaSeconds :type "Float (single-precision)"))
  (if (`self.NewVar`)
    (set `self.NewVar` true :!label _label)
    (if (not (<= (`/Game/FirstPerson/Blueprints/BP_FirstPersonCharacter.speed` (stale `self.Box.OnComponentBeginOverlap` _asbp_first_person_character)) 450.0))
      (`|ExecutionSequence`
        (:`then_0`
          (bind (_direction _newtrack_0) (`Timeline|Zaman Çizelgesi` :!label _label_2)
            (:`Update`
              (`SceneComponent.K2_SetRelativeLocation` (`self.Cube`) (`KismetMathLibrary.MakeVector` 0.0 0.0 (* _newtrack_0 -200.0)) false false))))
        (:`then_1`
          (`/Engine/EditorBlueprintResources/StandardMacros.DoOnce` false :!label _label_3
            (:`Completed`
              (`GameplayStatics.PlaySoundAtLocation` "/Game/music/doorsound.doorsound" (0.0 0.0 0.0) (struct) 1.0 1.0 0.0 null null null null)
              (if (not (stale `self.Box.OnComponentEndOverlap` _output_get))
                (goto _label_3 :!via `Reset`)))))))))

(event `self.Box.OnComponentBeginOverlap`
  (params (OverlappedComponent :type "PrimitiveComponent Object Reference") (OtherActor :type "Actor Object Reference") (OtherComp :type "PrimitiveComponent Object Reference") (OtherBodyIndex :type Integer) (bFromSweep :type Boolean) (SweepResult :type "HitResult Structure (by ref)"))
  (bind _asbp_first_person_character (cast `/Game/FirstPerson/Blueprints/BP_FirstPersonCharacter` OtherActor))
  (`|ExecutionSequence`
    (:`then_0`
      (goto _label))
    (:`then_1`
      (`/Engine/EditorBlueprintResources/StandardMacros.DoOnce` false
        (:`Completed`
          (`KismetSystemLibrary.Delay` 0.4)
          (`GameplayStatics.PlaySoundAtLocation` "/Game/speak/kapi9.kapi9" (`self.K2_GetActorLocation`) (struct) 1.0 1.0 0.0 null null null null)
          (`/Game/FirstPerson/Blueprints/BP_FirstPersonCharacter.7metin` _asbp_first_person_character))))))

(event `self.Box.OnComponentEndOverlap`
  (params (OverlappedComponent :type "PrimitiveComponent Object Reference") (OtherActor :type "Actor Object Reference") (OtherComp :type "PrimitiveComponent Object Reference") (OtherBodyIndex :type Integer))
  (cast `/Game/FirstPerson/Blueprints/BP_FirstPersonCharacter` OtherActor)
  (bind _output_get (set `self.NewVar` false))
  (`GameplayStatics.PlaySoundAtLocation` "/Game/music/doorsound.doorsound" (0.0 0.0 0.0) (struct) 1.0 1.0 0.0 null null null null)
  (goto _label_2 :!via `Reverse`))

(fn `UserConstructionScript`)