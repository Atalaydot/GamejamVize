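; One-shot trigger actor that spawns a light and starts a timed text and sound sequence when the first-person character enters its box.
; The box overlap casts to BP_FirstPersonCharacter, passes a DoOnce and spawns the Light class at a stored transform.
; After short and then long delays, it calls the character's Sirametin and 1metin ("metin" is Turkish for text), each followed by a sound at the trigger's location.
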(event `self.Box.OnComponentBeginOverlap`
  (params (OverlappedComponent :type "PrimitiveComponent Object Reference") (OtherActor :type "Actor Object Reference") (OtherComp :type "PrimitiveComponent Object Reference") (OtherBodyIndex :type Integer) (bFromSweep :type Boolean) (SweepResult :type "HitResult Structure (by ref)"))
  (bind _asbp_first_person_character (cast `/Game/FirstPerson/Blueprints/BP_FirstPersonCharacter` OtherActor))
  (`/Engine/EditorBlueprintResources/StandardMacros.DoOnce` false
    (:`Completed`
      (`|SpawnActorFromClass` "/Game/BluePrint/light/light.light_C" (`self.Spawn Transform`) "Undefined" "MultiplyWithRoot" null null)
      (`KismetSystemLibrary.Delay` 0.5)
      (`/Game/FirstPerson/Blueprints/BP_FirstPersonCharacter.sirametin` _asbp_first_person_character)
      (`GameplayStatics.PlaySoundAtLocation` "/Game/speak/1.1" (`self.K2_GetActorLocation`) (struct) 1.0 1.0 0.0 null null null null)
      (`KismetSystemLibrary.Delay` 16.0)
      (`/Game/FirstPerson/Blueprints/BP_FirstPersonCharacter.1metin` _asbp_first_person_character)
      (`GameplayStatics.PlaySoundAtLocation` "/Game/speak/2.2" (`self.K2_GetActorLocation`) (struct) 1.0 1.0 0.0 null null null null))))

(fn `UserConstructionScript`)