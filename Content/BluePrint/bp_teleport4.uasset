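; Trigger actor that starts a timed "15final" sequence when the first-person character enters Box1; despite its name, no teleport happens here.
; The overlap disables character movement and switches player 0 to UI-only input.
; Short delays then lead to the 15final sound at the actor's location and a call to the character's 15final.
; After a longer delay, it shows the mouse cursor.
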(event `self.Box1.OnComponentBeginOverlap`
  (params (OverlappedComponent :type "PrimitiveComponent Object Reference") (OtherActor :type "Actor Object Reference") (OtherComp :type "PrimitiveComponent Object Reference") (OtherBodyIndex :type Integer) (bFromSweep :type Boolean) (SweepResult :type "HitResult Structure (by ref)"))
  (bind _returnvalue (`GameplayStatics.GetPlayerController` 0))
  (bind _asbp_first_person_character (cast `/Game/FirstPerson/Blueprints/BP_FirstPersonCharacter` OtherActor))
  (`CharacterMovementComponent.DisableMovement` (`Character.CharacterMovement` _asbp_first_person_character))
  (`WidgetBlueprintLibrary.SetInputMode_UIOnlyEx` _returnvalue null)
  (`KismetSystemLibrary.Delay` 0.4)
  (`GameplayStatics.PlaySoundAtLocation` "/Game/speak/15final.15final" (`self.K2_GetActorLocation`) (struct) 1.0 1.0 0.0 null null null null)
  (`KismetSystemLibrary.Delay` 0.1)
  (`/Game/FirstPerson/Blueprints/BP_FirstPersonCharacter.15final` _asbp_first_person_character)
  (`KismetSystemLibrary.Delay` 3.7)
  (set `PlayerController.bShowMouseCursor` true _returnvalue))

(fn `UserConstructionScript`)